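; BP_Wall is a buildable fort wall that the player completes by striking it with a hammer.
; Each BP_Hammer overlap plays a hit sound and increments a counter.
; On the fifteenth hit the wall switches to wood materials, gains BlockAll collision and plays a success sound.
; After a short delay it finds the BP_Fort in the level and calls CheckComplete on it.
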(event `self.Wall_0.OnComponentBeginOverlap`
  (params (OverlappedComponent :type "PrimitiveComponent Object Reference") (OtherActor :type "Actor Object Reference") (OtherComp :type "PrimitiveComponent Object Reference") (OtherBodyIndex :type Integer) (bFromSweep :type Boolean) (SweepResult :type "HitResult Structure (by ref)"))
  (bind _wall_0 (`self.Wall_0`))
  (bind _hitcounter (`self.HitCounter`))
  (cast `/Game/Code/Blueprints/TheVladimir/BP_Hammer` OtherActor)
  (`GameplayStatics.PlaySound2D` "/Game/AssetsContent/Audio/Hammer_One.Hammer_One" 1.0 1.0 0.0 null null)
  (`/Engine/EditorBlueprintResources/StandardMacros.IncrementInt` _hitcounter
    (:`  `
      (if (== _hitcounter 15)
        (`PrimitiveComponent.SetMaterial` _wall_0 0 "/Game/ImportAssets/Fantastic_Village_Pack/materials/MI_wood_06.MI_wood_06")
        (`PrimitiveComponent.SetMaterial` _wall_0 1 "/Game/ImportAssets/Fantastic_Village_Pack/materials/MI_wood_detail_01.MI_wood_detail_01")
        (`PrimitiveComponent.SetCollisionProfileName` _wall_0 "BlockAll" true)
        (bind _returnvalue (`GameplayStatics.GetActorOfClass` "/Game/Code/Blueprints/TheVladimir/BP_Fort.BP_Fort_C"))
        (`GameplayStatics.PlaySound2D` "/Game/AssetsContent/Audio/Hammer_Successful.Hammer_Successful" 1.0 1.0 0.0 null null)
        (`KismetSystemLibrary.Delay` 2.0)
        (`/Game/Code/Blueprints/TheVladimir/BP_Fort.CheckComplete` _returnvalue)))))

(fn `UserConstructionScript`)