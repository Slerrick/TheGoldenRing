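; BP_Fort runs the fort-building task in the Vladimir level of an educational game about the Golden Gates and the city's defenses.
; On BeginPlay it fills its widget components with a Russian task panel and two two-answer history quizzes.
; Each CheckComplete call increments a building counter.
; At nine it plays a reward sound, waits briefly, then opens the Pereslavl level.
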(event `CheckComplete`
  (bind _result (`/Engine/EditorBlueprintResources/StandardMacros.IncrementInt` (`self.CounterOfBuildings`))
    (:`  `
      (if (== _result 9)
        (`GameplayStatics.PlaySound2D` "/Game/AssetsContent/Audio/Reward.Reward" 1.0 1.0 0.0 null null)
        (`KismetSystemLibrary.Delay` 6.0)
        (`GameplayStatics.OpenLevelBySoftObjectPtr` "/Game/Code/Maps/ThePereslavl.ThePereslavl")))))

(event `self.ReceiveBeginPlay`
  (bind _returnvalue (`|CreateWidget` "/Game/Code/Widgets/UMG_TaskTable.UMG_TaskTable_C" null "Золотые ворота Владимира — не только парадный вход, но и сложное фортификационное сооружение. Возведи пусть и деревянный, но крепкий оборонительный пункт. Можешь осмотреть и  Золотые ворота."))
  (`WidgetComponent.SetWidget` (`self.Task`) _returnvalue)
  (bind _returnvalue_2 (`|CreateWidget` "/Game/Code/Widgets/UMG_MiniTest.UMG_MiniTest_C" null "Какую роль выполняли Золотые ворота Владимира?" "Были только украшением и не имели отношения к обороне." "Служили парадным въездом и частью оборонительной системы города." false))
  (`WidgetComponent.SetWidget` (`self.Question_1`) _returnvalue_2)
  (bind _returnvalue_3 (`|CreateWidget` "/Game/Code/Widgets/UMG_MiniTest.UMG_MiniTest_C" null "Что окружало древний Владимир и помогало защищать его?" "Земляные валы и укреплённые ворота." "Каменная стена с электрическими воротами." true))
  (`WidgetComponent.SetWidget` (`self.Question_2`) _returnvalue_3))

(fn `UserConstructionScript`)