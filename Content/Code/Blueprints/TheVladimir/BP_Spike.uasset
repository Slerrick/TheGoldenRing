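; BP_Spike is a wooden spike that gets hammered in as part of building a fort.
; Each overlap with a BP_Hammer plays a hit sound and increments a counter.
; On the seventh hit it swaps to wood materials, switches collision to BlockAll and plays a success sound.
; After a short delay it asks the level's BP_Fort to check whether it is complete.
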(event `self.Spike_0.OnComponentBeginOverlap`
  (params (OverlappedComponent :type "PrimitiveComponent Object Reference") (OtherActor :type "Actor Object Reference") (OtherComp :type "PrimitiveComponent Object Reference") (OtherBodyIndex :type Integer) (bFromSweep :type Boolean) (SweepResult :type "HitResult Structure (by ref)"))
  (bind _spike_0 (`self.Spike_0`))
  (bind _hitcounter (`self.HitCounter`))
  (cast `/Game/Code/Blueprints/TheVladimir/BP_Hammer` OtherActor)
  (`GameplayStatics.PlaySound2D` "/Game/AssetsContent/Audio/Hammer_One.Hammer_One" 1.0 1.0 0.0 null null)
  (`/Engine/EditorBlueprintResources/StandardMacros.IncrementInt` _hitcounter
    (:`  `
      (if (== _hitcounter 7)
        (`PrimitiveComponent.SetMaterial` _spike_0 0 "/Game/ImportAssets/Fantastic_Village_Pack/materials/MI_wood_06.MI_wood_06")
        (`PrimitiveComponent.SetMaterial` _spike_0 1 "/Game/ImportAssets/Fantastic_Village_Pack/materials/MI_wood_detail_01.MI_wood_detail_01")
        (`PrimitiveComponent.SetCollisionProfileName` _spike_0 "BlockAll" true)
        (bind _returnvalue (`GameplayStatics.GetActorOfClass` "/Game/Code/Blueprints/TheVladimir/BP_Fort.BP_Fort_C"))
        (`GameplayStatics.PlaySound2D` "/Game/AssetsContent/Audio/Hammer_Successful.Hammer_Successful" 1.0 1.0 0.0 null null)
        (`KismetSystemLibrary.Delay` 2.0)
        (`/Engine/EditorBlueprintResources/StandardMacros.IsValid` _returnvalue
          (:`Is Valid`
            (`/Game/Code/Blueprints/TheVladimir/BP_Fort.CheckComplete` _returnvalue)))))))

(fn `UserConstructionScript`)