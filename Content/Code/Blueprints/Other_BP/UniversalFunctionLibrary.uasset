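; Blueprint function library with shared helpers for saved input scale, the saved Loud setting and the loading screen.
; GetInputScale reads the scale from its My_Save slot, defaulting to 1.0 when none exists.
; GetLoud doubles as getter and setter: with StartGame it loads or creates the save, otherwise it overwrites the stored value.
; ShowLoadScreen forwards the call to the My_Instance game instance.
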(fn `GetInputScale`
  (returns (inputscale :type "Float (double-precision)"))
  (bind _returnvalue (`GameplayStatics.DoesSaveGameExist` "InputScale"))
  (if _returnvalue
    (bind _returnvalue_2 (`GameplayStatics.LoadGameFromSlot` "InputScale"))
    (bind _asmy_save (cast `/Game/Code/My_Save` _returnvalue_2))
    (return (`/Game/Code/My_Save.VInputScale` _asmy_save))
    (else
      (return 1.0) ; If Android, Input scale must be between 0.1 and 0.5
    )))

(fn `GetLoud`
  (params (Loud :type "Float (double-precision)") (StartGame :type Boolean))
  (returns (NewLoud :type "Float (double-precision)"))
  (if StartGame
    (bind _returnvalue (`GameplayStatics.DoesSaveGameExist` "Loud"))
    (if _returnvalue
      (bind _returnvalue_2 (`GameplayStatics.LoadGameFromSlot` "Loud"))
      (bind _asmy_save (cast `/Game/Code/My_Save` _returnvalue_2))
      (return (`/Game/Code/My_Save.Loud` _asmy_save))
      (else
        (bind _returnvalue_3 (`GameplayStatics.CreateSaveGameObject` "/Game/Code/My_Save.My_Save_C"))
        (bind _output_get (set `/Game/Code/My_Save.Loud` Loud _returnvalue_3))
        (`GameplayStatics.SaveGameToSlot` _returnvalue_3 "Loud")
        (return _output_get)))
    (else
      (bind _returnvalue_4 (`GameplayStatics.LoadGameFromSlot` "Loud"))
      (bind _asmy_save_2 (cast `/Game/Code/My_Save` _returnvalue_4))
      (bind _output_get_2 (set `/Game/Code/My_Save.Loud` Loud _asmy_save_2))
      (`GameplayStatics.SaveGameToSlot` _returnvalue_4 "Loud")
      (return _output_get_2))))

(fn `ShowLoadScreen`
  (bind _asmy_instance (cast `/Game/Code/Blueprints/My_Instance` (`GameplayStatics.GetGameInstance` null)))
  (`/Game/Code/Blueprints/My_Instance.ShowLoadScreen` _asmy_instance)
  (return))