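; BP_GameMode is a game mode that plays a 2D guide sound for the current level shortly after play begins.
; After a short delay, it switches on the current level name, covering the menu and five levels such as The Syzdal and The Rostov.
; Each match passes an index to PlayGuide, which plays that entry from the Guides array.
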(event `self.ReceiveBeginPlay`
  (`KismetSystemLibrary.Delay` 2.5)
  (bind _returnvalue (`GameplayStatics.GetCurrentLevelName` true))
  (switch `string` _returnvalue
    (:`Menu`
      (`self.PlayGuide` 0))
    (:`TheSyzdal`
      (`self.PlayGuide` 1))
    (:`TheVladimir`
      (`self.PlayGuide` 2))
    (:`ThePereslavl`
      (`self.PlayGuide` 3))
    (:`TheRostov`
      (`self.PlayGuide` 4))
    (:`TheSergievPosad`
      (`self.PlayGuide` 5))))

(fn `PlayGuide`
  (params (Index :type Integer))
  (`GameplayStatics.PlaySound2D` (`|GetArrayItem` (`self.Guides`) Index) 1.0 1.0 0.0 null null))

(fn `UserConstructionScript`)