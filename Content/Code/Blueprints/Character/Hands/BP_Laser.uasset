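; BP_Laser is a hand laser pointer that clicks widgets and triggers BP_Kolokol actors.
; Press and Release drive the left mouse pointer key on its WidgetInteraction component.
; GetMeshData runs a short, debug-drawn visibility trace along that component's forward vector, calls OnLaserClick on a hit BP_Kolokol and returns whether one was found.
; A dynamic material on the Cylinder mesh, created at BeginPlay, lets SetLaserColor randomize the beam color.
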(event `self.ReceiveBeginPlay`
  (bind _cylinder (`self.Cylinder`))
  ;[0.02812 0.02812 0.02812] Get Laser Material
  (bind _returnvalue (`PrimitiveComponent.CreateDynamicMaterialInstance` _cylinder 0 (`PrimitiveComponent.GetMaterial` _cylinder 0) "Laser"))
  (set `self.LaserMaterial` _returnvalue))

(event `Press`
  ;[0.04062 0.04062 0.04062] Click on Widgets
  (`WidgetInteractionComponent.PressPointerKey` (`self.WidgetInteraction`) "LeftMouseButton"))

(event `Release`
  ;[0.04062 0.04062 0.04062] Click on Widgets
  (`WidgetInteractionComponent.ReleasePointerKey` (`self.WidgetInteraction`) "LeftMouseButton"))

(fn `Get Mesh Data`
  (returns (Succecful :type Boolean))
  (bind _widgetinteraction (`self.WidgetInteraction`))
  (bind _returnvalue (`SceneComponent.K2_GetComponentLocation` _widgetinteraction))
  (bind (_outhit _returnvalue_2) (`KismetSystemLibrary.LineTraceSingle` :`Start` _returnvalue :`End` (+ _returnvalue (* (`SceneComponent.GetForwardVector` _widgetinteraction) 450)) :`TraceChannel` "TraceTypeQuery1" :`DrawDebugType` "ForDuration"))
  (if _returnvalue_2
    (bind _asbp_kolokol (cast `/Game/Code/Blueprints/TheRostov/BP_Kolokol` (`.HitActor` (`GameplayStatics.BreakHitResult` _outhit)))
      (:`then`
        (`/Game/Code/Blueprints/TheRostov/BP_Kolokol.OnLaserClick` _asbp_kolokol)
        (if true
          (return true)
          (else
            _)))
      (:`CastFailed`
        _)))
  (return false))

(fn `SetLaserColor`
  (`MaterialInstanceDynamic.SetVectorParameterValue` (`self.LaserMaterial`) "LaserColor" (make `LinearColor` (`KismetMathLibrary.RandomFloat`) (`KismetMathLibrary.RandomFloat`) (`KismetMathLibrary.RandomFloat`) 1.0)))

(fn `UserConstructionScript`)