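; BP_Magnet is a pickup-style magnet actor that can also serve as the exit trigger to the TheRostov level.
; Any overlap with its DestroyZone plays a ping, as the VR_Player cast does not filter the overlapping actor.
; A regular magnet then destroys itself.
; One flagged IsFinal plays a reward sound, removes its DestroyZone and opens TheRostov after a short delay.
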(event `self.ReceiveBeginPlay`
  (set `self.Loc` (`SceneComponent.K2_GetComponentLocation` (`self.Magnet`))))

(event `self.DestroyZone.OnComponentBeginOverlap`
  (params (OverlappedComponent :type "PrimitiveComponent Object Reference") (OtherActor :type "Actor Object Reference") (OtherComp :type "PrimitiveComponent Object Reference") (OtherBodyIndex :type Integer) (bFromSweep :type Boolean) (SweepResult :type "HitResult Structure (by ref)"))
  (cast `/Game/Code/Blueprints/Character/VR_Player` OtherActor
    (:`then`
      _)
    (:`CastFailed`
      _))
  (`GameplayStatics.PlaySound2D` "/Engine/EngineSounds/1kSineTonePing.1kSineTonePing" 1.0 1.0 0.0 null null)
  (if (`self.IsFinal`)
    (`GameplayStatics.PlaySound2D` "/Game/AssetsContent/Audio/Reward.Reward" 1.0 1.0 0.0 null null)
    (`|ExecutionSequence`
      (:`then_0`
        (`ActorComponent.K2_DestroyComponent` (`self.DestroyZone`)))
      (:`then_1`
        (`KismetSystemLibrary.Delay` 6.0)
        (`GameplayStatics.OpenLevelBySoftObjectPtr` "/Game/Code/Maps/TheRostov.TheRostov")))
    (else
      (`self.K2_DestroyActor`))))

(fn `UserConstructionScript`)