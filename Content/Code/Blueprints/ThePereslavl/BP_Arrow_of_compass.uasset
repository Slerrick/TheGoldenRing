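; Compass arrow Blueprint that points horizontally at the nearest BP_Magnet in the level.
; A looping timed delay started on BeginPlay periodically rebuilds a cached list of every magnet's Loc value.
; Each Tick finds the closest cached location by squared distance and turns the Arrow component toward it on yaw only, zeroing pitch and roll.
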(event `self.ReceiveBeginPlay`
  (`KismetArrayLibrary.Array_Clear` (`self.All_Loc`) :!label _label)
  (bind _outactors (`GameplayStatics.GetAllActorsOfClass` "/Game/Code/Blueprints/ThePereslavl/BP_Magnet.BP_Magnet_C"))
  (for _array_element _outactors
    (`KismetArrayLibrary.Array_Add` (`self.All_Loc`) (`/Game/Code/Blueprints/ThePereslavl/BP_Magnet.Loc` _array_element)))
  (`KismetSystemLibrary.Delay` 0.2)
  (goto _label))

(event `self.ReceiveTick`
  (params (DeltaSeconds :type "Float (single-precision)"))
  (bind _all_loc (`self.All_Loc`))
  (bind (_returnvalue_roll _returnvalue_pitch _returnvalue_yaw) (`KismetMathLibrary.BreakRotator` (`KismetMathLibrary.FindLookAtRotation` (`self.ArrowLocation`) (`self.NearestMagnet`))))
  (if (`KismetArrayLibrary.Array_IsNotEmpty` _all_loc)
    (`|ExecutionSequence`
      (:`then_0`
        (set `self.NearestMagnet` (0.0 0.0 0.0))
        (set `self.NearestSqr` 999999999999.0)
        (set `self.ArrowLocation` (`SceneComponent.K2_GetComponentLocation` (`self.Arrow`)))
        (for _array_element _all_loc
          (bind _returnvalue (`KismetMathLibrary.VSizeSquared` (- _array_element (`self.ArrowLocation`))))
          (if (< _returnvalue (`self.NearestSqr`))
            (set `self.NearestMagnet` _array_element)
            (set `self.NearestSqr` _returnvalue))))
      (:`then_1`
        (`SceneComponent.K2_SetWorldRotation` (`self.Arrow`) (`KismetMathLibrary.MakeRotator` 0.0 0.0 _returnvalue_yaw) false false)))))

(fn `UserConstructionScript`)