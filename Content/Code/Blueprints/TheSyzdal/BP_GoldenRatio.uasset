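; Golden-ratio jigsaw puzzle for the Suzdal level, where physics-simulated sprite pieces snap into nine target slots.
; Each slot's overlap calls SnapPuzzels, which matches the piece's second component tag to the slot index, then freezes and aligns that sprite with a ping.
; When all nine are placed, Reward plays a sound and, after a delay, opens TheVladimir level.
; BeginPlay fills a task widget with the Russian puzzle instructions.
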(event `self.Puzzle_0.OnComponentBeginOverlap`
  (params (OverlappedComponent :type "PrimitiveComponent Object Reference") (OtherActor :type "Actor Object Reference") (OtherComp :type "PrimitiveComponent Object Reference") (OtherBodyIndex :type Integer) (bFromSweep :type Boolean) (SweepResult :type "HitResult Structure (by ref)"))
  (bind _goldenratio_sprite_0 (`self.GoldenRatio_Sprite_0`))
  (`/Engine/EditorBlueprintResources/StandardMacros.IsValid` OtherComp
    (:`Is Valid`
      (bind _successful (`self.SnapPuzzels` 0 OtherComp))
      (if _successful
        (`PrimitiveComponent.SetSimulatePhysics` _goldenratio_sprite_0 false)
        (`PrimitiveComponent.SetCollisionProfileName` _goldenratio_sprite_0 "NoCollision" true)
        (`SceneComponent.K2_SetWorldLocationAndRotation` _goldenratio_sprite_0 (`SceneComponent.K2_GetComponentLocation` (`self.Puzzle_0`)) (struct :`Roll` -90.0) false false)
        (`GameplayStatics.PlaySound2D` "/Engine/EngineSounds/1kSineTonePing.1kSineTonePing" 1.0 1.0 0.0 null null :!label _label)))))

(event `self.Puzzle_1.OnComponentBeginOverlap`
  (params (OverlappedComponent :type "PrimitiveComponent Object Reference") (OtherActor :type "Actor Object Reference") (OtherComp :type "PrimitiveComponent Object Reference") (OtherBodyIndex :type Integer) (bFromSweep :type Boolean) (SweepResult :type "HitResult Structure (by ref)"))
  (bind _goldenratio_sprite_1 (`self.GoldenRatio_Sprite_1`))
  (`/Engine/EditorBlueprintResources/StandardMacros.IsValid` OtherComp
    (:`Is Valid`
      (bind _successful (`self.SnapPuzzels` 1 OtherComp))
      (if _successful
        (`PrimitiveComponent.SetSimulatePhysics` _goldenratio_sprite_1 false)
        (`PrimitiveComponent.SetCollisionProfileName` _goldenratio_sprite_1 "NoCollision" true)
        (`SceneComponent.K2_SetWorldLocationAndRotation` _goldenratio_sprite_1 (`SceneComponent.K2_GetComponentLocation` (`self.Puzzle_1`)) (struct :`Roll` -90.0) false false)
        (goto _label)))))

(event `self.Puzzle_2.OnComponentBeginOverlap`
  (params (OverlappedComponent :type "PrimitiveComponent Object Reference") (OtherActor :type "Actor Object Reference") (OtherComp :type "PrimitiveComponent Object Reference") (OtherBodyIndex :type Integer) (bFromSweep :type Boolean) (SweepResult :type "HitResult Structure (by ref)"))
  (bind _goldenratio_sprite_2 (`self.GoldenRatio_Sprite_2`))
  (`/Engine/EditorBlueprintResources/StandardMacros.IsValid` OtherComp
    (:`Is Valid`
      (bind _successful (`self.SnapPuzzels` 2 OtherComp))
      (if _successful
        (`PrimitiveComponent.SetSimulatePhysics` _goldenratio_sprite_2 false)
        (`PrimitiveComponent.SetCollisionProfileName` _goldenratio_sprite_2 "NoCollision" true)
        (`SceneComponent.K2_SetWorldLocationAndRotation` _goldenratio_sprite_2 (`SceneComponent.K2_GetComponentLocation` (`self.Puzzle_2`)) (struct :`Roll` -90.0) false false)
        (goto _label)))))

(event `self.Puzzle_3.OnComponentBeginOverlap`
  (params (OverlappedComponent :type "PrimitiveComponent Object Reference") (OtherActor :type "Actor Object Reference") (OtherComp :type "PrimitiveComponent Object Reference") (OtherBodyIndex :type Integer) (bFromSweep :type Boolean) (SweepResult :type "HitResult Structure (by ref)"))
  (bind _goldenratio_sprite_3 (`self.GoldenRatio_Sprite_3`))
  (`/Engine/EditorBlueprintResources/StandardMacros.IsValid` OtherComp
    (:`Is Valid`
      (bind _successful (`self.SnapPuzzels` 3 OtherComp))
      (if _successful
        (`PrimitiveComponent.SetSimulatePhysics` _goldenratio_sprite_3 false)
        (`PrimitiveComponent.SetCollisionProfileName` _goldenratio_sprite_3 "NoCollision" true)
        (`SceneComponent.K2_SetWorldLocationAndRotation` _goldenratio_sprite_3 (`SceneComponent.K2_GetComponentLocation` (`self.Puzzle_3`)) (struct :`Roll` -90.0) false false)
        (goto _label)))))

(event `self.Puzzle_4.OnComponentBeginOverlap`
  (params (OverlappedComponent :type "PrimitiveComponent Object Reference") (OtherActor :type "Actor Object Reference") (OtherComp :type "PrimitiveComponent Object Reference") (OtherBodyIndex :type Integer) (bFromSweep :type Boolean) (SweepResult :type "HitResult Structure (by ref)"))
  (bind _goldenratio_sprite_4 (`self.GoldenRatio_Sprite_4`))
  (`/Engine/EditorBlueprintResources/StandardMacros.IsValid` OtherComp
    (:`Is Valid`
      (bind _successful (`self.SnapPuzzels` 4 OtherComp))
      (if _successful
        (`PrimitiveComponent.SetSimulatePhysics` _goldenratio_sprite_4 false)
        (`PrimitiveComponent.SetCollisionProfileName` _goldenratio_sprite_4 "NoCollision" true)
        (`SceneComponent.K2_SetWorldLocationAndRotation` _goldenratio_sprite_4 (`SceneComponent.K2_GetComponentLocation` (`self.Puzzle_4`)) (struct :`Roll` -90.0) false false)
        (goto _label)))))

(event `self.Puzzle_5.OnComponentBeginOverlap`
  (params (OverlappedComponent :type "PrimitiveComponent Object Reference") (OtherActor :type "Actor Object Reference") (OtherComp :type "PrimitiveComponent Object Reference") (OtherBodyIndex :type Integer) (bFromSweep :type Boolean) (SweepResult :type "HitResult Structure (by ref)"))
  (bind _goldenratio_sprite_5 (`self.GoldenRatio_Sprite_5`))
  (`/Engine/EditorBlueprintResources/StandardMacros.IsValid` OtherComp
    (:`Is Valid`
      (bind _successful (`self.SnapPuzzels` 5 OtherComp))
      (if _successful
        (`PrimitiveComponent.SetSimulatePhysics` _goldenratio_sprite_5 false)
        (`PrimitiveComponent.SetCollisionProfileName` _goldenratio_sprite_5 "NoCollision" true)
        (`SceneComponent.K2_SetWorldLocationAndRotation` _goldenratio_sprite_5 (`SceneComponent.K2_GetComponentLocation` (`self.Puzzle_5`)) (struct :`Roll` -90.0) false false)
        (goto _label)))))

(event `self.Puzzle_6.OnComponentBeginOverlap`
  (params (OverlappedComponent :type "PrimitiveComponent Object Reference") (OtherActor :type "Actor Object Reference") (OtherComp :type "PrimitiveComponent Object Reference") (OtherBodyIndex :type Integer) (bFromSweep :type Boolean) (SweepResult :type "HitResult Structure (by ref)"))
  (bind _goldenratio_sprite_6 (`self.GoldenRatio_Sprite_6`))
  (`/Engine/EditorBlueprintResources/StandardMacros.IsValid` OtherComp
    (:`Is Valid`
      (bind _successful (`self.SnapPuzzels` 6 OtherComp))
      (if _successful
        (`PrimitiveComponent.SetSimulatePhysics` _goldenratio_sprite_6 false)
        (`PrimitiveComponent.SetCollisionProfileName` _goldenratio_sprite_6 "NoCollision" true)
        (`SceneComponent.K2_SetWorldLocationAndRotation` _goldenratio_sprite_6 (`SceneComponent.K2_GetComponentLocation` (`self.Puzzle_6`)) (struct :`Roll` -90.0) false false)
        (goto _label)))))

(event `self.Puzzle_7.OnComponentBeginOverlap`
  (params (OverlappedComponent :type "PrimitiveComponent Object Reference") (OtherActor :type "Actor Object Reference") (OtherComp :type "PrimitiveComponent Object Reference") (OtherBodyIndex :type Integer) (bFromSweep :type Boolean) (SweepResult :type "HitResult Structure (by ref)"))
  (bind _goldenratio_sprite_7 (`self.GoldenRatio_Sprite_7`))
  (`/Engine/EditorBlueprintResources/StandardMacros.IsValid` OtherComp
    (:`Is Valid`
      (bind _successful (`self.SnapPuzzels` 7 OtherComp))
      (if _successful
        (`PrimitiveComponent.SetSimulatePhysics` _goldenratio_sprite_7 false)
        (`PrimitiveComponent.SetCollisionProfileName` _goldenratio_sprite_7 "NoCollision" true)
        (`SceneComponent.K2_SetWorldLocationAndRotation` _goldenratio_sprite_7 (`SceneComponent.K2_GetComponentLocation` (`self.Puzzle_7`)) (struct :`Roll` -90.0) false false)
        (goto _label)))))

(event `self.Puzzle_8.OnComponentBeginOverlap`
  (params (OverlappedComponent :type "PrimitiveComponent Object Reference") (OtherActor :type "Actor Object Reference") (OtherComp :type "PrimitiveComponent Object Reference") (OtherBodyIndex :type Integer) (bFromSweep :type Boolean) (SweepResult :type "HitResult Structure (by ref)"))
  (bind _goldenratio_sprite_8 (`self.GoldenRatio_Sprite_8`))
  (`/Engine/EditorBlueprintResources/StandardMacros.IsValid` OtherComp
    (:`Is Valid`
      (bind _successful (`self.SnapPuzzels` 8 OtherComp))
      (if _successful
        (`PrimitiveComponent.SetSimulatePhysics` _goldenratio_sprite_8 false)
        (`PrimitiveComponent.SetCollisionProfileName` _goldenratio_sprite_8 "NoCollision" true)
        (`SceneComponent.K2_SetWorldLocationAndRotation` _goldenratio_sprite_8 (`SceneComponent.K2_GetComponentLocation` (`self.Puzzle_8`)) (struct :`Roll` -90.0) false false)
        (goto _label)))))

(event `Reward`
  (`GameplayStatics.PlaySound2D` "/Game/AssetsContent/Audio/Reward.Reward" 1.0 1.0 0.0 null null)
  (`KismetSystemLibrary.Delay` 6.0)
  (`GameplayStatics.OpenLevelBySoftObjectPtr` "/Game/Code/Maps/TheVladimir.TheVladimir"))

(event `self.ReceiveBeginPlay`
  (bind _returnvalue (`|CreateWidget` "/Game/Code/Widgets/UMG_TaskTable.UMG_TaskTable_C" null "В Суздале красота храмов и колоколен начинается с точного расчёта. Зодчие продумывали пропорции, чтобы части здания складывались в гармоничное целое. Собери пазл золотого сечения."))
  (`WidgetComponent.SetWidget` (`self.Task`) _returnvalue))

(fn `CheckComplete`
  (if (== (`self.CounterSuccessful`) 9)
    (`self.Reward`)))

(fn `SnapPuzzels`
  (params (Index :type Integer) (ActorComp :type "ActorComponent Object Reference"))
  (returns (Successful :type Boolean))
  (if (`ActorComponent.ComponentHasTag` ActorComp "Puzzle")
    (if (== Index (`KismetStringLibrary.Conv_StringToInt` (`KismetStringLibrary.Conv_NameToString` (`|GetArrayItem` (`ActorComponent.ComponentTags` ActorComp) 1))))
      (`/Engine/EditorBlueprintResources/StandardMacros.IncrementInt` (`self.CounterSuccessful`)
        (:`  `
          (`self.CheckComplete`)
          (return true)))
      (else
        (return false)))
    (else
      (return false))))

(fn `UserConstructionScript`)