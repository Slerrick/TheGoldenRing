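; A clickable bell (kolokol) for a bell puzzle, played by laser click and checked against a BP_PlayOnKolokoles manager found at BeginPlay.
; A click, ignored while locked or while the truth sequence plays, sends the bell's ID to the manager's CheckComplete.
; Success plays the bell animation and its unique sound with a short cooldown, while failure plays an error sound.
; PlaySequence triggers the same animation and sound without the check.
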(event `self.ReceiveBeginPlay`
  (bind _returnvalue (`GameplayStatics.GetActorOfClass` "/Game/Code/Blueprints/TheRostov/BP_PlayOnKolokoles.BP_PlayOnKolokoles_C"))
  (set `self.AllKolokoles` _returnvalue))

(event `PlaySequence`
  (`SkeletalMeshComponent.PlayAnimation` (`self.Kolokol`) "/Game/AssetsContent/Props/TheRostov/Kolokol_Anim_Bell_Move.Kolokol_Anim_Bell_Move" false)
  (`GameplayStatics.PlaySound2D` (`self.UniqSound`) 1.0 1.0 1.0 null null))

(event `OnLaserClick`
  (if (and (`self.CanClick?`) (not (`self.TruthSequencePlaying?`)))
    (set `self.CanClick?` false)
    (bind _successful (`/Game/Code/Blueprints/TheRostov/BP_PlayOnKolokoles.CheckComplete` (`self.AllKolokoles`) (`self.ID`)))
    (if _successful
      (`SkeletalMeshComponent.PlayAnimation` (`self.Kolokol`) "/Game/AssetsContent/Props/TheRostov/Kolokol_Anim_Bell_Move.Kolokol_Anim_Bell_Move" false)
      (`GameplayStatics.PlaySound2D` (`self.UniqSound`) 1.0 1.0 1.0 null null)
      (`KismetSystemLibrary.Delay` 1.5)
      (set `self.CanClick?` true)
      (else
        (`GameplayStatics.PlaySound2D` "/Engine/EditorSounds/Notifications/CompileFailed.CompileFailed" 1.0 1.0 0.0 null null)
        (set `self.CanClick?` true)))))

(fn `UserConstructionScript`)