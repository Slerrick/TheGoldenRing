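; Bell-ringing memory puzzle in the Rostov level: the player hears a bell sequence and repeats it, with a task widget explaining the goal.
; BeginPlay indexes BP_Kolokol actors by ID; ListenSequence uses MultiGates to select one of three sequences and play its four bells on timed delays.
; CheckComplete validates each bell ID and calls NewSequence on completion, which re-enables listening or, after the third, plays a reward and opens TheSergievPosad.
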(event `self.ReceiveBeginPlay`
  (bind _outactors (`GameplayStatics.GetAllActorsOfClass` "/Game/Code/Blueprints/TheRostov/BP_Kolokol.BP_Kolokol_C"))
  (for _array_element _outactors
    (`KismetArrayLibrary.Array_Set` (`self.Kolokoles`) (`/Game/Code/Blueprints/TheRostov/BP_Kolokol.ID` _array_element) _array_element))
  (bind _returnvalue (`|CreateWidget` "/Game/Code/Widgets/UMG_TaskTable.UMG_TaskTable_C" null "Ростов Великий славится колокольными звонами, а каждый колокол обладает своим голосом. На его звучание влияют форма и металл, а чистый тон рождается благодаря точному литью и резонансу. Вслушайся в последовательность ударов и повтори её."))
  (`WidgetComponent.SetWidget` (`self.Task`) _returnvalue))

(event `ListenSequence`
  (`KismetSystemLibrary.Delay` 1.0)
  (if (`self.canListen?`)
    (set `self.canListen?` false)
    (`|MultiGate` false
      (:`Out 0`
        (set `self.currentSequence` (`self.Sequence_0`)))
      (:`Out 1`
        (set `self.currentSequence` (`self.Sequence_1`)))
      (:`Out 2`
        (set `self.currentSequence` (`self.Sequence_2`))))
    (bind _result (`/Engine/EditorBlueprintResources/StandardMacros.IncrementInt` (`self.currentKolokolPlay`) :!label _label)
      (:`  `
        (`|MultiGate` false :!label _label_2
          (:`Out 0`
            _)
          (:`Out 1`
            _)
          (:`Out 2`
            _)
          (:`Out 3`
            _)
          (:`Out 4`
            (for _array_element (`self.Kolokoles`)
              (set `/Game/Code/Blueprints/TheRostov/BP_Kolokol.TruthSequencePlaying?` false _array_element))
            (set `self.currentKolokolPlay` 0)
            (goto _label_2 :!via `Reset`)))
        (`self.PlayOnID` _result)
        (`KismetSystemLibrary.Delay` 1.5)
        (goto _label)))))

(event `NewSequence`
  (`|MultiGate` false
    (:`Out 0`
      (set `self.canListen?` true :!label _label_3)
      (for _array_element (`self.Kolokoles`)
        (set `/Game/Code/Blueprints/TheRostov/BP_Kolokol.TruthSequencePlaying?` true _array_element)
        (set `self.currentKolokolPlay` -1))
      (`GameplayStatics.PlaySound2D` "/Game/AssetsContent/Audio/CompileSuccess.CompileSuccess" 1.0 1.0 0.0 null null))
    (:`Out 1`
      (goto _label_3))
    (:`Out 2`
      (`GameplayStatics.PlaySound2D` "/Game/AssetsContent/Audio/Reward.Reward" 1.0 1.0 0.0 null null)
      (`KismetSystemLibrary.Delay` 6.0)
      (`GameplayStatics.OpenLevelBySoftObjectPtr` "/Game/Code/Maps/TheSergievPosad.TheSergievPosad"))))

(fn `CheckComplete`
  (params (ID :type Integer))
  (returns (Successful :type Boolean))
  (if (== ID (`|GetArrayItem` (`self.currentSequence`) (`self.currentKolokolPlay`)))
    (if (== (`self.currentKolokolPlay`) 3)
      (for _array_element (`self.Kolokoles`)
        (set `/Game/Code/Blueprints/TheRostov/BP_Kolokol.TruthSequencePlaying?` true _array_element))
      (`self.NewSequence`)
      (return true)
      (else
        (`/Engine/EditorBlueprintResources/StandardMacros.IncrementInt` (`self.currentKolokolPlay`)
          (:`  `
            (return true)))))
    (else
      (return false))))

(fn `PlayOnID`
  (params (Sequence_part :type Integer))
  (`/Game/Code/Blueprints/TheRostov/BP_Kolokol.PlaySequence` (`|GetArrayItem` (`self.Kolokoles`) (`|GetArrayItem` (`self.currentSequence`) Sequence_part))))

(fn `UserConstructionScript`)