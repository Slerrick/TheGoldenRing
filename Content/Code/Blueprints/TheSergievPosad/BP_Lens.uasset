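; BP_Lens is a lens that focuses sunlight into a visible fire point on surfaces.
; Each tick it compares its Arrow direction with a sun vector cached at BeginPlay, then line-traces from FocusPoint toward the sun for obstructions.
; When clear, a short Arrow trace moves FirePoint to the impact.
; Paired DoOnce gates toggle visibility, hiding it only on misalignment, not on blocked sun or missed trace.
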(event `self.ReceiveBeginPlay`
  (set `self.IncomingVector` (`KismetMathLibrary.NegateVector` (`KismetMathLibrary.GetForwardVector` (`self.SunVectorRot`)))))

(event `self.ReceiveTick`
  (params (DeltaSeconds :type "Float (single-precision)"))
  (bind _returnvalue (`SceneComponent.K2_GetComponentLocation` (`self.FocusPoint`)))
  (bind _returnvalue_2 (`SceneComponent.K2_GetComponentLocation` (`self.Arrow`)))
  (set `self.ArrowVector` (`SceneComponent.GetForwardVector` (`self.Arrow`)))
  (if (> (`KismetMathLibrary.Dot_VectorVector` (`self.IncomingVector`) (`KismetMathLibrary.NegateVector` (`self.ArrowVector`))) 0.85)
    (bind (_outhit _returnvalue_3) (`KismetSystemLibrary.LineTraceSingle` _returnvalue (+ _returnvalue (* (`self.IncomingVector`) 5000)) "TraceTypeQuery1"))
    (if (not _returnvalue_3)
      (set `self.RayStart` _returnvalue_2)
      (set `self.RayEnd` (+ _returnvalue_2 (* (`self.ArrowVector`) 300)))
      (bind (_outhit_2 _returnvalue_4) (`KismetSystemLibrary.LineTraceSingle` (`self.RayStart`) (`self.RayEnd`) "TraceTypeQuery1"))
      (if _returnvalue_4
        (`SceneComponent.K2_SetWorldLocation` (`self.FirePoint`) (`.ImpactPoint` (`GameplayStatics.BreakHitResult` _outhit_2)) false false)
        (`/Engine/EditorBlueprintResources/StandardMacros.DoOnce` false :!label _label
          (:`Completed`
            (`SceneComponent.SetVisibility` (`self.FirePoint`) true false)
            (`self.ResetVisF`)))))
    (else
      (`/Engine/EditorBlueprintResources/StandardMacros.DoOnce` false :!label _label_2
        (:`Completed`
          (`SceneComponent.SetVisibility` (`self.FirePoint`) false false)
          (`self.ResetVisT`))))))

(event `ResetVisT`
  (goto _label :!via `Reset`))

(event `ResetVisF`
  (goto _label_2 :!via `Reset`))

(fn `UserConstructionScript`)