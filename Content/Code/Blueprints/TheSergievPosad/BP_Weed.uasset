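; BP_Weed is a weed actor that is destroyed by sustained contact with a burning BP_PointFire, apparently as part of a weed-clearing task.
; Overlap events on its Straw component set the burn state when the fire mesh is visible and clear it when contact ends.
; A looping timer accumulates burn for about five seconds, resetting when interrupted, then notifies BP_WeedCounter, plays a sound and destroys the weed.
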(event `self.ReceiveBeginPlay`
  (`KismetSystemLibrary.K2_SetTimerDelegate` (delegate `CheckBurn`) 0.1 true)
  (bind _returnvalue (`GameplayStatics.GetActorOfClass` "/Game/Code/Blueprints/TheSergievPosad/BP_WeedCounter.BP_WeedCounter_C"))
  (set `self.WeedCounter` _returnvalue))

(event `CheckBurn`
  (if (`self.Is_Burn?`)
    (bind _result (`/Engine/EditorBlueprintResources/StandardMacros.IncrementInt` (`self.LevelBurn`))
      (:`  `
        (if (> _result 50)
          (`/Game/Code/Blueprints/TheSergievPosad/BP_WeedCounter.CheckComplete` (`self.WeedCounter`))
          (`GameplayStatics.PlaySound2D` "/Engine/VREditor/Sounds/UI/Foliage_Placed.Foliage_Placed" 1.0 1.0 0.0 null null)
          (`self.K2_DestroyActor`))))
    (else
      (set `self.LevelBurn` 0))))

(event `self.Straw.OnComponentBeginOverlap`
  (params (OverlappedComponent :type "PrimitiveComponent Object Reference") (OtherActor :type "Actor Object Reference") (OtherComp :type "PrimitiveComponent Object Reference") (OtherBodyIndex :type Integer) (bFromSweep :type Boolean) (SweepResult :type "HitResult Structure (by ref)"))
  (bind _asbp_point_fire (cast `/Game/Code/Blueprints/TheSergievPosad/BP_PointFire` OtherActor))
  (if (`SceneComponent.IsVisible` (`/Game/Code/Blueprints/TheSergievPosad/BP_PointFire.FireMesh` _asbp_point_fire))
    (set `self.Is_Burn?` true)))

(event `self.Straw.OnComponentEndOverlap`
  (params (OverlappedComponent :type "PrimitiveComponent Object Reference") (OtherActor :type "Actor Object Reference") (OtherComp :type "PrimitiveComponent Object Reference") (OtherBodyIndex :type Integer))
  (cast `/Game/Code/Blueprints/TheSergievPosad/BP_PointFire` OtherActor)
  (set `self.Is_Burn?` false))

(fn `UserConstructionScript`)