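; BP_WeedCounter tracks completion of the Sergiev Posad grass-burning task, where the player angles a lens to focus sunlight on grass until it ignites.
; On BeginPlay it fills its Task widget component with a UMG_TaskTable showing the Russian instructions.
; Each CheckComplete call increments Counter; once it exceeds seven, a reward sound plays and, after a short delay, the Final level opens.
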(event `CheckComplete`
  (bind _result (`/Engine/EditorBlueprintResources/StandardMacros.IncrementInt` (`self.Counter`))
    (:`  `
      (if (> _result 7)
        (`GameplayStatics.PlaySound2D` "/Game/AssetsContent/Audio/Reward.Reward" 1.0 1.0 0.0 null null)
        (`KismetSystemLibrary.Delay` 6.0)
        (`GameplayStatics.OpenLevelBySoftObjectPtr` "/Game/Code/Maps/Final.Final")))))

(event `self.ReceiveBeginPlay`
  (bind _returnvalue (`|CreateWidget` "/Game/Code/Widgets/UMG_TaskTable.UMG_TaskTable_C" null "В Сергиевом Посаде точность мастера важна даже в простых действиях. Наклони линзу под нужным углом к солнцу и направь собранный ею пучок света на траву. Подбери положение, при котором луч сфокусируется в одной точке и трава загорится."))
  (`WidgetComponent.SetWidget` (`self.Task`) _returnvalue))

(fn `UserConstructionScript`)